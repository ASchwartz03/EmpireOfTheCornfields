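; Stand-in enemy that attacks Troop1 and BP_HERO actors entering its ActiveArea sphere, which is sized by Range around its spawn point.
; Overlaps queue targets in Troops and play a timeline used as a tick, damaging the first at close range whenever a countdown expires.
; DecreaseHealth and a duplicate SuperHero function lower its health, update the text display and destroy it at zero.
; Random wandering logic exists but is unconnected.
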(event `self.ReceiveBeginPlay`
  (add `PrimitiveComponent.OnComponentBeginOverlap` (`self.activeArea`) (delegate `attackTroop`)))

(event `attackTroop`
  (params (OverlappedComponent :type "PrimitiveComponent Object Reference") (OtherActor :type "Actor Object Reference") (OtherComp :type "PrimitiveComponent Object Reference") (OtherBodyIndex :type Integer) (bFromSweep :type Boolean) (SweepResult :type "HitResult Structure (by ref)"))
  (bind _output (`|GetArrayItem` (`self.troops`)))
  (bind _astroop_1 (cast `/Game/Interface/Troops/Troop1` OtherActor)
    (:`then`
      (`KismetArrayLibrary.Array_AddUnique` (`self.troops`) _astroop_1)
      (`Timeline|attackTroopTick` :!label _label
        (:`Update`
          (`/Engine/EditorBlueprintResources/StandardMacros.IsValid` _output
            (:`Is Valid`
              (if (not (> (`KismetMathLibrary.Vector_Distance` (`self.K2_GetActorLocation`) (`self.K2_GetActorLocation` _output)) 120.0))
                (bind _result (`/Engine/EditorBlueprintResources/StandardMacros.DecrementInt` (`self.attackCooldown`))
                  (:`  `
                    (if (<= _result 0)
                      (`/Game/Interface/Troops/Troop1.decreaseHealth` (`|GetArrayItem` (`self.troops`)) 10)
                      (set `self.attackCooldown` (`self.maxAttackCooldown`)))))))
            (:`Is Not Valid`
              (`TimelineComponent.Stop` (`self.attackTroopTick`))
              (`KismetArrayLibrary.Array_Remove` (`self.troops`)))))))
    (:`CastFailed`
      (bind _asbp_hero (cast `/Game/Interface/Troops/BP_HERO` OtherActor))
      (`KismetArrayLibrary.Array_AddUnique` (`self.troops`) _asbp_hero)
      (goto _label))))

(fn `decreaseHealth`
  (params (amount :type Integer))
  (bind _output_get (set `self.health` (- (`self.health`) amount)))
  (`TextRenderComponent.K2_SetText` (`self.TextRender`) (`KismetTextLibrary.Conv_IntToText` _output_get))
  (if (<= (`self.health`) 0)
    (`self.K2_DestroyActor`)))

(fn `Super Hero`
  (params (Amount :type Integer))
  (bind _output_get (set `self.health` (- (`self.health`) Amount)))
  (`TextRenderComponent.K2_SetText` (`self.TextRender`) (`KismetTextLibrary.Conv_IntToText` _output_get))
  (if (<= (`self.health`) 0)
    (`self.K2_DestroyActor`)))

(fn `UserConstructionScript`
  (bind _output_get (set `self.spawnLoc` (`self.K2_GetActorLocation`)))
  (`SceneComponent.K2_SetWorldLocation` (`self.activeArea`) _output_get false false)
  (`SphereComponent.SetSphereRadius` (`self.activeArea`) (`self.range`) true))