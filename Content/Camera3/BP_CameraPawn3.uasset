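; Player camera pawn for an RTS on a hex grid, handling bounded pan and pitch-linked zoom, selection, building and troop orders.
; A camera-forward trace selects actors and flags them as builder, hero or building through interfaces, gating construction, the hero attack and spawn menu.
; A per-tick trace feeds the BuildingManager cursor, while game mode inventories gate previews and pay for construction.
; Selected units move via BP_troopMover, and troops spawn near the selected building.
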(event Custom|SpawnMenu
  (bind _buildingname (CallFunction|SelectableCheck))
  (Variables|Default|SetName%20for%20Menu _buildingname))

(event Custom|Get%20Selected%20Building%20Value
  (params (Name :type Name))
  (bind _got_name_for_selected (CallFunction|SelectedNameFunct Name))
  (Variables|Default|SetGot%20Name%20for%20Selected _got_name_for_selected))

(event Custom|Spawn%20At%20Building
  (params (Troop%20Name :type Name))
  (bind _buildingselectableref (Variables|Default|GetBuildingSelectableRef))
  (bind _returnvalue (Transformation|GetActorTransform _buildingselectableref))
  (Development|PrintString (Utilities|String|ToString(Name) Troop%20Name))
  (if (== Troop%20Name "Spear")
    (Game|SpawnActorfromClass "/Game/Interface/Troops/Troop1.Troop1_C" (Math|Transform|MakeTransform (Math|Vector|MakeVector (+ (.x (.location _returnvalue)) (Math|Random|RandomFloatinRange 1e+02 4.5e+02)) (+ (.y (.location _returnvalue)) (Math|Random|RandomFloatinRange 1e+02 4.5e+02)) (.z (.location _returnvalue))) "0, 0, 0" "1.000000,1.000000,1.000000") "Undefined" "MultiplyWithRoot" 0 0 :!label _label)
    (elif (== Troop%20Name "Gunner")
      (goto _label)
      (elif (== Troop%20Name "Tank")
        (goto _label)
        (else
          (Development|PrintString "no building name"))))))

(event Input|EnhancedActionEvents|EnhancedInputActionIA_SpawnMenu
  (params (ActionValue :type Boolean) (ElapsedSeconds :type Float%20%28double-precision%29) (TriggeredSeconds :type Float%20%28double-precision%29) (InputAction :type Input%20Action%20Object%20Reference :default "/Game/Camera3/Inputs/MenuWidgets/IA_SpawnMenu.IA_SpawnMenu"))
  (:Started
    (if (Variables|Building|Bool|GetBuilding%20Selected)
      (bind _array_element (Utilities|Array|ForEachLoopwithBreak (Variables|Camera|GetSelectedActor))
        (:LoopBody
          (bind _asbp_building_selectable (Utilities|Casting|CastToBP_BuildingSelectable _array_element))
          (Variables|Default|SetBuildingSelectableRef _asbp_building_selectable)
          (Utilities|IsValid (Variables|Default|GetBuildingSelectableRef)
            (:Is%20Valid
              (CallFunction|GetSelectedBuildingValue (Variables|/Game/Building/Buildings/BP_BuildingSelectable.BP_BuildingSelectable_C|GetBuilding%20Built%20Name _asbp_building_selectable))
              (bind _foundwidgets (Widget|GetAllWidgetsOfClass "/Game/Building/Widgets/WBP_MainUI.WBP_MainUI_C" true))
              (bind _array_element_2 (Utilities|Array|ForEachLoopwithBreak _foundwidgets)
                (:LoopBody
                  (Default|SpawnCalled _array_element_2 (Variables|Building|Bool|GetBuilding%20Selected) (Variables|Default|GetGot%20Name%20for%20Selected)))))))))))

(event Input|EnhancedActionEvents|EnhancedInputActionIA_troopMove2
  (params (ActionValue :type Boolean) (ElapsedSeconds :type Float%20%28double-precision%29) (TriggeredSeconds :type Float%20%28double-precision%29) (InputAction :type Input%20Action%20Object%20Reference :default "/Game/Camera3/Inputs/IA_troopMove2.IA_troopMove2"))
  ;[1 1 1] Move Unit
  (Utilities|IsValid (Variables|References|GettroopMover)
    (:Is%20Valid
      _)
    (:Is%20Not%20Valid
      (bind _returnvalue (Game|SpawnActorfromClass "/Game/TroopMover/BP_troopMover.BP_troopMover_C" (Math|Transform|MakeTransform "0, 0, 0" "0, 0, 0" "1.000000,1.000000,1.000000") "Undefined" "MultiplyWithRoot" 0 0))
      (Variables|References|SettroopMover _returnvalue)))
  (Default|GiveCommand (Variables|References|GettroopMover) (Variables|Camera|GetSelectedActor) self))

(event Input|EnhancedActionEvents|EnhancedInputActionIA_Move
  (params (ActionValue :type Vector%202D%20Structure) (ElapsedSeconds :type Float%20%28double-precision%29) (TriggeredSeconds :type Float%20%28double-precision%29) (InputAction :type Input%20Action%20Object%20Reference :default "/Game/Camera3/Inputs/IA_Move.IA_Move"))
  ;[1 1 1] Camera Move
  (CameraZoom|MoveCamera ActionValue))

(event Input|EnhancedActionEvents|EnhancedInputActionIA_Zoom
  (params (ActionValue :type Float%20%28double-precision%29) (ElapsedSeconds :type Float%20%28double-precision%29) (TriggeredSeconds :type Float%20%28double-precision%29) (InputAction :type Input%20Action%20Object%20Reference :default "/Game/Camera3/Inputs/IA_Zoom.IA_Zoom"))
  ;[1 1 1] Camera Zoom
  (CameraZoom|ZoomCamera ActionValue))

(event Input|EnhancedActionEvents|EnhancedInputActionIA_PrimaryAction
  (params (ActionValue :type Boolean) (ElapsedSeconds :type Float%20%28double-precision%29) (TriggeredSeconds :type Float%20%28double-precision%29) (InputAction :type Input%20Action%20Object%20Reference :default "/Game/Camera3/Inputs/IA_PrimaryAction.IA_PrimaryAction"))
  ;[1 1 1] Switch To Construction
  (if (Variables|Camera|GetBuilderSelected)
    (Development|PrintString (Utilities|String|ToString(Name) (Variables|References|GetBuilding%20Name)))
    (switch Utilities|FlowControl|Switch|SwitchonEPrimaryActionModes (Variables|Inputs|GetActionMode)
      (:NewEnumerator1
        (CallFunction|MinusMaterials)
        (Buildings|Construction|ConstructionEvents)))))

(event EventUpdateGameSpeed
  (params (NewSpeedMultipier :type Float%20%28double-precision%29))
  ;[1 1 1] Update Game Speed
  (Class|BPIGameTime|UpdateGameSpeed(Message) (Game|GetGameState) NewSpeedMultipier))

(event EventBeginPlay
  ;[1 1 1] Place Cursor In View Port
  (bind _returnvalue (Actor|GetActorOfClass "/Game/Camera3/GMB_Camera3.GMB_Camera3_C"))
  (Variables|References|SetGamemode _returnvalue)
  (bind _returnvalue_2 (UserInterface|CreateWidget "/Game/Interface/CrossHairTestUI.CrossHairTestUI_C"))
  (UserInterface|Viewport|AddtoViewport _returnvalue_2 0)
  (CameraZoom|Initialize))

(event EventTick
  (params (DeltaSeconds :type Float%20%28single-precision%29))
  ;[1 1 1] Set Cursor Position
  (bind _output_get (Variables|Camera|SetCursorPosition (Inputs|SetBuildPosition (+ (CameraZoom|GetCurrentArmLength) 2e+03))))
  (Default|SetCursorPosition (Variables|Default|GetBuildingManager) _output_get))

(event EventSetDateTime
  (params (DateTimeStruct :type Date%20Time%20Structure))
  ;[1 1 1] Set Date Time
  (Class|BPIGameTime|SetDateTime(Message) (Variables|References|GetMainWidgetRef) DateTimeStruct))

(event EventSetGameSpeedInt
  (params (GameSpeed :type Float%20%28double-precision%29))
  ;[1 1 1] Set Game Speed
  (Class|BPIGameTime|SetGameSpeedInt(Message) (Variables|References|GetMainWidgetRef) GameSpeed))

(event EventStartPreview
  (params (RowName :type Name :default "None"))
  ;[1 1 1] Start Preview
  (if (Default|GetIsPreviewing (Variables|Default|GetBuildingManager))
    (Default|DestoryPreview (Variables|Default|GetBuildingManager)))
  (Default|SetPreview (Variables|Default|GetBuildingManager) RowName)
  (Inputs|SetActionMode "NewEnumerator0"))

(event Input|KeyboardEvents|B
  (params (Key :type Key%20Structure :default "None"))
  (bind _buildingmanager (Variables|Default|GetBuildingManager))
  (bind _buildingmanager_2 (Variables|Default|GetBuildingManager))
  (bind _bispreviewing (Default|GetIsPreviewing _buildingmanager))
  ;[1 1 1] Controls For Build Function
  (:Pressed
    (if (Variables|Camera|GetBuilderSelected)
      (Utilities|FlowControl|FlipFlop
        (:A
          (if (not _bispreviewing)
            (bind _returnvalue (CallFunction|BarracksCheck :!label _label))
            (if _returnvalue
              (Default|SetPreview _buildingmanager_2 (Variables|References|GetBuilding%20Name))
              (Inputs|SetActionMode "NewEnumerator1")
              (else
                (bind _returnvalue_2 (CallFunction|SiloCheck))
                (if _returnvalue_2
                  (Default|SetPreview _buildingmanager_2 (Variables|References|GetBuilding%20Name))
                  (Inputs|SetActionMode "NewEnumerator1")
                  (else
                    (bind _returnvalue_3 (CallFunction|GarageCheck))
                    (if _returnvalue_3
                      (Default|SetPreview _buildingmanager_2 (Variables|References|GetBuilding%20Name))
                      (Inputs|SetActionMode "NewEnumerator1"))))))))
        (:B
          (if _bispreviewing
            (Default|DestoryPreview _buildingmanager_2 :!label _label_2)
            (else
              (goto _label)))))
      (else
        (goto _label_2)))))

(event Input|KeyboardEvents|SpaceBar
  (params (Key :type Key%20Structure :default "None"))
  (bind _returnvalue (Game|GetPlayerCameraManager 0))
  (bind _selectedactor (Variables|Camera|GetSelectedActor))
  (bind _returnvalue_2 (Camera|GetCameraLocation _returnvalue))
  ;[1 1 1] Line Trace for Selection
  (:Pressed
    (bind (_outhit _returnvalue_3) (Collision|LineTraceForObjects _returnvalue_2 (+ _returnvalue_2 (* (Transformation|GetActorForwardVector _returnvalue) "2500.000000,2500.000000,2500.000000")) (Utilities|Array|MakeArray "ObjectTypeQuery2") false (Variables|References|GetignoreActors) "ForOneFrame"))
    ;[1 1 1] Selected
    (if (and _returnvalue_3 (Utilities|DoesObjectImplementInterface (.hitactor _outhit) "/Game/Interface/SelectActorInterface.SelectActorInterface_C"))
      (Utilities|Array|AddUnique _selectedactor (.hitactor _outhit))
      (Class|SelectActorInterface|SelectMyActor(Message) (.hitactor _outhit))
      (if (Utilities|DoesObjectImplementInterface (.hitactor _outhit) "/Game/Interface/BuildInterface.BuildInterface_C")
        (Variables|Camera|SetBuilderSelected true))
      (if (Utilities|DoesObjectImplementInterface (.hitactor _outhit) "/Game/Interface/BP_HeroInterface.BP_HeroInterface_C")
        (Variables|Camera|SetHeroSelected true))
      (if (Utilities|DoesObjectImplementInterface (.hitactor _outhit) "/Game/Interface/BPI_Building.BPI_Building_C")
        (Variables|Building|Bool|SetBuilding%20Selected true))
      (for _array_element (Variables|Camera|GetSelectedActor)
        _)
      (else
        ;[1 1 1] Deselected
        (bind _isselected_ (Class|SelectActorInterface|IsSelected(Message) (.hitactor _outhit)))
        (if (not _isselected_)
          (Class|SelectActorInterface|DeselectMyActor(Message) _selectedactor)
          (Variables|Camera|SetHeroSelected false)
          (Variables|Camera|SetBuilderSelected false)
          (Variables|Building|Bool|SetBuilding%20Selected false)
          (for _array_element_2 (Variables|Camera|GetSelectedActor)
            (Utilities|Array|Clear (Variables|Camera|GetSelectedActor))))))))

(event Input|KeyboardEvents|CapsLock
  (params (Key :type Key%20Structure :default "None"))
  ;[1 1 1] Hero Power Move
  (:Pressed
    (if (Variables|Camera|GetHeroSelected)
      (bind _returnvalue (Actor|GetActorOfClass "/Game/TemporaryStandinClasses/BP_attackThis.BP_attackThis_C"))
      (Default|DecreaseHealth _returnvalue 20))))

(fn ConstructionScript)

(fn MoveCamera
  (params (actionValue :type Vector%202D%20Structure))
  (bind _returnvalue (Transformation|GetActorLocation))
  (bind _cameraspeed (Variables|Camera|GetcameraSpeed))
  (bind _minloc (Variables|Camera|GetminLoc))
  (bind _maxloc (Variables|Camera|GetmaxLoc))
  (bind _springarm (Variables|Default|GetSpringArm))
  (bind _targetarmlength (Variables|/Script/Engine.SpringArmComponent|GetTargetArmLength _springarm))
  (bind _returnvalue_2 (* actionValue _cameraspeed _targetarmlength))
  (bind _returnvalue_3 (Math|Conversions|ToVector(Vector2D) _returnvalue_2))
  (bind _returnvalue_4 (+ _returnvalue _returnvalue_3))
  (Transformation|SetActorLocation (Math|Vector|MakeVector (Math|Float|Clamp(Float) (.x _returnvalue_4) (.x _minloc) (.x _maxloc)) (Math|Float|Clamp(Float) (.y _returnvalue_4) (.y _minloc) (.y _maxloc)) (.z _returnvalue_4)) false false))

(fn ZoomCamera
  (params (actionValue :type Float%20%28double-precision%29))
  (bind _springarm (Variables|Default|GetSpringArm))
  ;[1 1 1] Zoom
  (Variables|/Script/Engine.SpringArmComponent|SetTargetArmLength _springarm (|(clamp((currentLength*((input*{9EF2F684-4D24-658D-0B90-BAA2996449D2})+1)),{48BC9623-4987-0C27-71D0-2883A42EBD03},{52024120-437B-68C5-25DD-5AA5B50BA5BB})) (Variables|/Script/Engine.SpringArmComponent|GetTargetArmLength (Variables|Default|GetSpringArm)) actionValue))
  (Transformation|SetRelativeRotation _springarm (Math|Rotator|MakeRotator 0.0 (|(lerp({00F330BD-4770-0FDA-0C1C-66B09124047A},{16ADD25A-4BF6-7DBA-7546-778CE10B35DF},((currentLength-{48BC9623-4987-0C27-71D0-2883A42EBD03})/({52024120-437B-68C5-25DD-5AA5B50BA5BB}-{48BC9623-4987-0C27-71D0-2883A42EBD03})))) (Variables|/Script/Engine.SpringArmComponent|GetTargetArmLength (Variables|Default|GetSpringArm))) -9e+01) false false))

(fn Initialize
  ;[1 1 1] set up input
  (Input|AddMappingContext (PlayerController|LocalPlayerSubsystems|GetEnhancedInputLocalPlayerSubsystem (Game|GetPlayerController 0)) "/Game/Camera3/Inputs/IMC_Camera3.IMC_Camera3" 0 "(bIgnoreAllPressedKeysUntilRelease=True,bForceImmediately=False,bNotifyUserSettings=False)")
  ;[1 1 1] find map bounds
  (bind _returnvalue (Actor|GetActorOfClass "/Game/Map_Grid/BP_HexGrid.BP_HexGrid_C"))
  (Transformation|SetActorLocation (+ (Transformation|GetActorLocation _returnvalue) "0.000000,0.000000,-250.000000") false false)
  (Variables|Camera|SetminLoc (Utilities|Operators|Subtract (.Origin (Collision|GetActorBounds _returnvalue false false)) (.BoxExtent (Collision|GetActorBounds _returnvalue false false)) "-90.000000,-40.000000,0.000000"))
  (Variables|Camera|SetmaxLoc (+ (.Origin (Collision|GetActorBounds _returnvalue false false)) (.BoxExtent (Collision|GetActorBounds _returnvalue false false)) "-100.000000,-110.000000,0.000000"))
  ;[1 1 1] initialize other variables
  (Variables|Camera|SetcameraSpeed 0.02)
  (Variables|Camera|SetzoomSpeed 0.1)
  (Variables|Camera|SetminZoom 8e+02)
  (Variables|Camera|SetmaxZoom 2e+03)
  (Variables|Camera|SetminYaw -5e+01)
  (Variables|Camera|SetmaxYaw -3e+01)
  (Variables|/Script/Engine.SpringArmComponent|SetTargetArmLength (Variables|Default|GetSpringArm) (Math|Float|Lerp (Variables|Camera|GetminZoom) (Variables|Camera|GetmaxZoom) 0.5))
  ;[1 1 1] move camera in bounds and set yaw to match zoom
  (CameraZoom|ZoomCamera 0.0)
  (CameraZoom|MoveCamera)
  (bind _outactors (Actor|GetAllActorsOfClass "/Game/TemporaryStandinClasses/BP_attackThis.BP_attackThis_C"))
  (Variables|References|SetignoreActors _outactors))

(fn GetCurrentArmLength
  (return (Variables|/Script/Engine.SpringArmComponent|GetTargetArmLength (Variables|Default|GetSpringArm))))

(fn SetBuildPosition
  (params (Trace%20Distance :type Float%20%28double-precision%29))
  (bind _returnvalue (Game|GetPlayerCameraManager 0))
  (bind _returnvalue_2 (Camera|GetCameraLocation _returnvalue))
  (bind _outhit (Collision|LineTraceByChannel _returnvalue_2 (+ _returnvalue_2 (* (Transformation|GetActorForwardVector _returnvalue) Trace%20Distance)) "TraceTypeQuery1" false 0 "None"))
  (Utilities|Casting|CastToBP_HexGrid (.HitActor (Collision|BreakHitResult _outhit)))
  (return (.Location (Collision|BreakHitResult _outhit))))

(fn GetGridSnaps)

(fn SetActionMode
  (params (ActionMode :type EPrimaryActionModes%20Enum :default "NewEnumerator0"))
  (Variables|Inputs|SetActionMode ActionMode)
  (return))

(fn ConstructionChecks
  (bind _buildingmanager (Variables|Default|GetBuildingManager))
  (if (Default|GetIsPreviewValid (Variables|Default|GetBuildingManager))
    (if (and (not (Default|GetIsPreviewOverlapping _buildingmanager)) (not (Default|GetIsPreviewonSlope _buildingmanager)))
      ;[1 1 1] Checking if the player has enough resources
      (if true
        (return true)
        (else
          _))))
  (return false))

(fn RemovePreview
  (bind _buildingmanager (Variables|Default|GetBuildingManager))
  (Default|StoreVariables _buildingmanager)
  (Default|DestoryPreview _buildingmanager))

(fn ConstructionEvents
  (bind _validbuild (Buildings|Construction|ConstructionChecks))
  (if _validbuild
    (Buildings|Construction|RemovePreview)
    (Default|SpawnConstruction (Variables|Default|GetBuildingManager))
    (Inputs|SetActionMode "NewEnumerator0")))

(fn BarracksCheck
  (bind _returnvalue (Actor|GetActorOfClass "/Game/Camera3/GMB_Camera3.GMB_Camera3_C"))
  (return (Math|Boolean|ANDBoolean (>= (Variables|/Game/Camera3/GMB_Camera3.GMB_Camera3_C|GetBeerInventory _returnvalue) 6) (>= (Variables|/Game/Camera3/GMB_Camera3.GMB_Camera3_C|GetCashInventory _returnvalue) 6) (Variables|Building|Bool|GetBarracks!))))

(fn SiloCheck
  (bind _returnvalue (Actor|GetActorOfClass "/Game/Camera3/GMB_Camera3.GMB_Camera3_C"))
  (return (Math|Boolean|ANDBoolean (>= (Variables|/Game/Camera3/GMB_Camera3.GMB_Camera3_C|GetBeerInventory _returnvalue) 16) (>= (Variables|/Game/Camera3/GMB_Camera3.GMB_Camera3_C|GetCashInventory _returnvalue) 16) (Variables|Building|Bool|GetSilo!))))

(fn GarageCheck
  (bind _returnvalue (Actor|GetActorOfClass "/Game/Camera3/GMB_Camera3.GMB_Camera3_C"))
  (return (Math|Boolean|ANDBoolean (>= (Variables|/Game/Camera3/GMB_Camera3.GMB_Camera3_C|GetBeerInventory _returnvalue) 22) (>= (Variables|/Game/Camera3/GMB_Camera3.GMB_Camera3_C|GetCashInventory _returnvalue) 22) (>= (Variables|/Game/Camera3/GMB_Camera3.GMB_Camera3_C|GetDipInventory _returnvalue) 22) (Variables|Building|Bool|GetGarage!))))

(fn MinusMaterials
  (bind _gamemode (Variables|References|GetGamemode))
  (bind _gamemode_2 (Variables|References|GetGamemode))
  (bind _gamemode_3 (Variables|References|GetGamemode))
  (if (Variables|Building|Bool|GetBarracks!)
    (Variables|/Game/Camera3/GMB_Camera3.GMB_Camera3_C|SetBeerInventory _gamemode_3 (- (Variables|/Game/Camera3/GMB_Camera3.GMB_Camera3_C|GetBeerInventory _gamemode_3) 18))
    (Variables|/Game/Camera3/GMB_Camera3.GMB_Camera3_C|SetCashInventory _gamemode_3 (- (Variables|/Game/Camera3/GMB_Camera3.GMB_Camera3_C|GetCashInventory _gamemode_3) 18))
    (elif (Variables|Building|Bool|GetSilo!)
      (Variables|/Game/Camera3/GMB_Camera3.GMB_Camera3_C|SetBeerInventory _gamemode_2 (- (Variables|/Game/Camera3/GMB_Camera3.GMB_Camera3_C|GetBeerInventory _gamemode_2) 12))
      (Variables|/Game/Camera3/GMB_Camera3.GMB_Camera3_C|SetCashInventory _gamemode_2 (- (Variables|/Game/Camera3/GMB_Camera3.GMB_Camera3_C|GetCashInventory _gamemode_2) 12))
      (elif (Variables|Building|Bool|GetGarage!)
        (Variables|/Game/Camera3/GMB_Camera3.GMB_Camera3_C|SetBeerInventory _gamemode (- (Variables|/Game/Camera3/GMB_Camera3.GMB_Camera3_C|GetBeerInventory _gamemode) 22))
        (Variables|/Game/Camera3/GMB_Camera3.GMB_Camera3_C|SetCashInventory _gamemode (- (Variables|/Game/Camera3/GMB_Camera3.GMB_Camera3_C|GetCashInventory _gamemode) 22))
        (Variables|/Game/Camera3/GMB_Camera3.GMB_Camera3_C|SetDipInventory _gamemode (- (Variables|/Game/Camera3/GMB_Camera3.GMB_Camera3_C|GetDipInventory _gamemode) 22))))))

(fn SetPreviewOfBuilding
  (params (self2 :type BP%20Building%20Manager%20Object%20Reference) (self3 :type BP%20Building%20Manager%20Object%20Reference) (self4 :type BP%20Building%20Manager%20Object%20Reference))
  (bind _returnvalue (CallFunction|BarracksCheck))
  (if _returnvalue
    (Default|SetPreview self2 (Variables|References|GetBuilding%20Name))
    (Inputs|SetActionMode "NewEnumerator1")
    (else
      (bind _returnvalue_2 (CallFunction|SiloCheck))
      (if _returnvalue_2
        (Default|SetPreview self3 (Variables|References|GetBuilding%20Name))
        (Inputs|SetActionMode "NewEnumerator1")
        (else
          (bind _returnvalue_3 (CallFunction|GarageCheck))
          (if _returnvalue_3
            (Default|SetPreview self4 (Variables|References|GetBuilding%20Name))
            (Inputs|SetActionMode "NewEnumerator1")))))))

(fn SelectableCheck
  (if (== (Variables|References|GetBuilding%20Name) "Barracks")
    (bind _output_get (Variables|References|SetBuilding%20Name "Barracks"))
    (return _output_get)
    (elif (== (Variables|References|GetBuilding%20Name) "Silo")
      (bind _output_get_2 (Variables|References|SetBuilding%20Name "Silo"))
      (return _output_get_2)
      (elif (== (Variables|References|GetBuilding%20Name) "Garage")
        (bind _output_get_3 (Variables|References|SetBuilding%20Name "Garage"))
        (return _output_get_3)))))

(fn SelectedNameFunct
  (params (Name :type Name))
  (if (Variables|Building|Bool|GetBuilding%20Selected)
    (if (== Name "Barracks")
      (bind _output_get (Variables|Default|SetSelected%20Name "Barracks"))
      (return _output_get)
      (elif (== Name "Silo")
        (bind _output_get_2 (Variables|Default|SetSelected%20Name "Silo"))
        (return _output_get_2)
        (elif (== Name "Garage")
          (bind _output_get_3 (Variables|Default|SetSelected%20Name "Garage"))
          (return _output_get_3)
          (else
            (Development|PrintString "no building name")))))))

(fn GetGameState
  (return 0))