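; BP_Trailer is a building that acts as a drop-off point for builders carrying resource B.
; The construction script centers the ActiveArea sphere on the actor and sizes it from Range.
; When a BP_Builder holding the resource begins overlapping that area, a short one-shot timer starts, then calls Gather2 on that builder.
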(event `self.ReceiveBeginPlay`
  ;[1 1 1] Bind Overlap Event
  (add `PrimitiveComponent.OnComponentBeginOverlap` (`self.activeArea`) (delegate `DropOff`)))

(event `DropOff`
  (params (OverlappedComponent :type "PrimitiveComponent Object Reference") (OtherActor :type "Actor Object Reference") (OtherComp :type "PrimitiveComponent Object Reference") (OtherBodyIndex :type Integer) (bFromSweep :type Boolean) (SweepResult :type "HitResult Structure (by ref)"))
  ;[1 1 1] Drop Off Event
  (bind _asbp_builder (cast `/Game/Interface/Troops/BP_Builder` OtherActor))
  (if (`/Game/Interface/Troops/BP_Builder.HasResourceB?` _asbp_builder)
    (bind _returnvalue (`KismetSystemLibrary.K2_SetTimerDelegate` (delegate `DropOffLoop`) 2.0))
    (set `self.Drop Timer` _returnvalue)))

(event `DropOffLoop`
  ;[1 1 1] Drop Off Event
  (`/Game/Interface/Troops/BP_Builder.Gather2` (stale `DropOff` _asbp_builder)))

(fn `UserConstructionScript`
  ;[1 1 1] Construction
  (bind _output_get (set `self.spawnLoc` (`self.K2_GetActorLocation`)))
  (`SceneComponent.K2_SetWorldLocation` (`self.activeArea`) _output_get false false)
  (`SphereComponent.SetSphereRadius` (`self.activeArea`) (`self.range`) true))