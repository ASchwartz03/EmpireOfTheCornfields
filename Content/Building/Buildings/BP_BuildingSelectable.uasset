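; BP_BuildingSelectable is a building actor that shows the mesh for whichever building type was built.
; Its Selectable event stores the passed name and picks the Barracks, Silo or Garage static mesh through chained name comparisons, printing a debug message for any other name.
; IsSelected is a stub that always returns false, and the construction script is empty.
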(event `Selectable`
  (params (BuildingBuilt :type Name))
  ;[1 1 1] Set Static Mesh for BuildingSelectable
  (bind _output_get (set `self.Building Built Name` BuildingBuilt))
  (if (== _output_get "Barracks")
    (set `self.Building Built Name` "Barracks")
    (`StaticMeshComponent.SetStaticMesh` (`self.CurrentBuildingMesh`) "/Game/Building/Meshes/Buildings/Barracks/Barn3.Barn3")
    (elif (== _output_get "Silo")
      (set `self.Building Built Name` "Silo")
      (`StaticMeshComponent.SetStaticMesh` (`self.CurrentBuildingMesh`) "/Game/Building/Meshes/Buildings/Silo/Silo3.Silo3")
      (elif (== _output_get "Garage")
        (set `self.Building Built Name` "Garage")
        (`StaticMeshComponent.SetStaticMesh` (`self.CurrentBuildingMesh`) "/Game/Building/Meshes/Buildings/Garage/Garage3.Garage3")
        (else
          (`KismetSystemLibrary.PrintString` "no name"))))))

(fn `IsSelected`
  (returns (`isselected?` :type Boolean))
  (return false))

(fn `UserConstructionScript`)