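; BP_BeerNode is a beer resource node that builder units harvest by entering its range.
; Construction centers the ActiveArea sphere on the actor and sizes it from Range.
; A BP_Builder overlap stores that builder and starts a one-shot timer, which adds Beer to the stored builder and calls its DropOff.
; It keeps only the latest builder and has no end-overlap handling.
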(event `self.ReceiveBeginPlay`
  ;[1 1 1] Overlap Event
  (add `PrimitiveComponent.OnComponentBeginOverlap` (`self.activeArea`) (delegate `GatherBeer`)))

(event `GatherBeer`
  (params (OverlappedComponent :type "PrimitiveComponent Object Reference") (OtherActor :type "Actor Object Reference") (OtherComp :type "PrimitiveComponent Object Reference") (OtherBodyIndex :type Integer) (bFromSweep :type Boolean) (SweepResult :type "HitResult Structure (by ref)"))
  ;[1 1 1] Gather Beer
  (bind _asbp_builder (cast `/Game/Interface/Troops/BP_Builder` OtherActor))
  (set `self.BuilderUnit` _asbp_builder)
  (bind _returnvalue (`KismetSystemLibrary.K2_SetTimerDelegate` (delegate `GatherBeerLoop`) 4.0))
  (set `self.BeerTimer` _returnvalue))

(event `GatherBeerLoop`
  (bind _builderunit (`self.BuilderUnit`))
  ;[1 1 1] Beer Loop
  (set `/Game/Interface/Troops/BP_Builder.Beer` (+ (`/Game/Interface/Troops/BP_Builder.Beer` _builderunit) 6) _builderunit)
  (bind _output_get (set `self.NameOfResource` "Beer"))
  (`/Game/Interface/Troops/BP_Builder.Drop Off` _builderunit _output_get))

(fn `UserConstructionScript`
  ;[1 1 1] Construct
  (bind _output_get (set `self.spawnLoc` (`self.K2_GetActorLocation`)))
  (`SceneComponent.K2_SetWorldLocation` (`self.activeArea`) _output_get false false)
  (`SphereComponent.SetSphereRadius` (`self.activeArea`) (`self.range`) true))