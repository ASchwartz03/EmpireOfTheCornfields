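; BP_DipNode is a resource node where builder units gather Dip.
; A builder entering the ActiveArea sphere, centred on the actor and sized by Range at construction, starts a one-shot timer.
; When the timer fires, it adds a fixed amount of Dip to the stored builder and calls its DropOff with the resource name.
; Only one builder reference and timer handle are kept, overwritten on each new overlap.
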(event `self.ReceiveBeginPlay`
  ;[1 1 1] Block Overlap
  (add `PrimitiveComponent.OnComponentBeginOverlap` (`self.activeArea`) (delegate `GatherDip`)))

(event `GatherDip`
  (params (OverlappedComponent :type "PrimitiveComponent Object Reference") (OtherActor :type "Actor Object Reference") (OtherComp :type "PrimitiveComponent Object Reference") (OtherBodyIndex :type Integer) (bFromSweep :type Boolean) (SweepResult :type "HitResult Structure (by ref)"))
  ;[1 1 1] Gather Dip
  (bind _asbp_builder (cast `/Game/Interface/Troops/BP_Builder` OtherActor))
  (set `self.BuilderUnit` _asbp_builder)
  (bind _returnvalue (`KismetSystemLibrary.K2_SetTimerDelegate` (delegate `GatherDipLoop`) 4.0))
  (set `self.DipTimer` _returnvalue))

(event `GatherDipLoop`
  (bind _builderunit (`self.BuilderUnit`))
  ;[1 1 1] Dip Loop
  (set `/Game/Interface/Troops/BP_Builder.Dip` (+ (`/Game/Interface/Troops/BP_Builder.Dip` _builderunit) 6) _builderunit)
  (bind _output_get (set `self.NameOfResource` "Dip"))
  (`/Game/Interface/Troops/BP_Builder.Drop Off` _builderunit _output_get))

(fn `UserConstructionScript`
  (bind _output_get (set `self.spawnLoc` (`self.K2_GetActorLocation`)))
  (`SceneComponent.K2_SetWorldLocation` (`self.activeArea`) _output_get false false)
  (`SphereComponent.SetSphereRadius` (`self.activeArea`) (`self.range`) true))