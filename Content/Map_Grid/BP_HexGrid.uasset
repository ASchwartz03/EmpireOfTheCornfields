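; Hex-grid map generator that lays out staggered rows of tiles in its construction script, spaced from the tile mesh bounds.
; Tiles are either mesh instances or BP_Tile child actors, chosen by the Instanced flag.
; Instances get random water or land heights, also written to per-instance custom data; child actors stay flat.
; Two FastNoise wrappers are configured, but their noise sampling is disconnected, so heights ignore the noise settings.
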(fn `UserConstructionScript`
  (locals (`Instance Index` :type Integer :default 0))
  (bind _returnvalue (`KismetMathLibrary.RandomFloatInRange` -1.0 1.0))
  ;[1 1 1] Construct Noise Level 1
  (bind _returnvalue_2 (`|GenericCreateObject` "/Script/FastNoiseGenerator.FastNoiseWrapper"))
  (bind _output_get (set `self.Noise Wrapper Lv 1` _returnvalue_2))
  (`FastNoiseWrapper.SetupFastNoise` _output_get (`self.Noise Type`) (`self.Seed`) (`self.Frequency`) (`self.Interp`) (`self.Fractaltype`) (`self.Octaves`) (`self.Lacunarity`) (`self.Gain`) (`self.Cellular Jitter`) (`self.Cellular Distance Function`) (`self.Cellular Return Type`))
  ;[1 1 1] Construct Noise Level 2
  (bind _returnvalue_3 (`|GenericCreateObject` "/Script/FastNoiseGenerator.FastNoiseWrapper"))
  (bind _output_get_2 (set `self.Noise Wrapper 2` _returnvalue_3))
  (`FastNoiseWrapper.SetupFastNoise` _output_get_2 (`self.Noise Type_2`) (`self.Seed_2`) (`self.Frequency_2`) (`self.Interp_2`) (`self.Fractaltype_2`) (`self.Octaves_2`) (`self.Lacunarity_2`) (`self.Gain_2`) (`self.Cellular Jitter_2`) (`self.Cellular Distance Function_2`) (`self.2 Cellular Return Type_0`))
  (`StaticMeshComponent.SetStaticMesh` (`self.InstancedStaticMesh`) (`self.Tile Mesh`))
  (set `self.Radius` (* (`self.Scale`) (.x (`.Max` (break `Box` (`StaticMesh.GetBoundingBox` (`self.Tile Mesh`)))))))
  ;[1 1 1] Height Loop
  (for _index (range (`self.Height`))
    ;[1 1 1] Width Loop
    (for _index_2 (range (`self.Width`))
      (if (`self.Instanced?`)
        (bind _returnvalue_4 (+ (* _index_2 (`self.Radius`) 2.0) (* (`self.Offset`) _index_2) (`self.RowOffset`)))
        (bind _returnvalue_5 (+ (* (/ (* (`self.Radius`) 2.0) (`KismetMathLibrary.Sqrt` 3.0)) 1.5 _index) (* (`self.Offset`) _index)))
        ;[1 1 1] Instanced Mesh
        (bind _returnvalue_6 (`InstancedStaticMeshComponent.AddInstance` (`self.InstancedStaticMesh`) (`KismetMathLibrary.MakeTransform` (`KismetMathLibrary.MakeVector` _returnvalue_4 _returnvalue_5) (struct) (`KismetMathLibrary.Conv_DoubleToVector` (`self.Scale`))) false))
        ;[1 1 1] Instance Height Calculator
        (set `local.Instance Index` _returnvalue_6)
        (if (<= _returnvalue 0.0)
          (set `self.Tile Height` (`self.Base Water Height`))
          (else
            (set `self.Tile Height` (`KismetMathLibrary.FClamp` _returnvalue 0.1))))
        (`InstancedStaticMeshComponent.UpdateInstanceTransform` (`self.InstancedStaticMesh`) (`local.Instance Index`) (`KismetMathLibrary.MakeTransform` (+ (.location (`InstancedStaticMeshComponent.GetInstanceTransform` (`self.InstancedStaticMesh`) (`local.Instance Index`) true)) (`KismetMathLibrary.MakeVector` 0.0 0.0 (+ (`self.Tile Height Offset`) (* (`self.Tile Height`) (`self.Tile Height Strength`)))))) false false false)
        (`InstancedStaticMeshComponent.SetCustomDataValue` (`self.InstancedStaticMesh`) (`local.Instance Index`) 0 (`self.Tile Height`) true)
        (else
          ;[1 1 1] Child Actors
          (bind _returnvalue_7 (`AddComponent|NODE_AddChildActorComponent-0` :`RelativeTransform` (`KismetMathLibrary.MakeTransform` (`KismetMathLibrary.MakeVector` _returnvalue_4 _returnvalue_5) (struct) (`KismetMathLibrary.Conv_DoubleToVector` (`self.Scale`)))))
          (`ChildActorComponent.SetChildActorClass` _returnvalue_7 "/Game/Map_Grid/BP_Tile.BP_Tile_C"))))
    (`/Engine/EditorBlueprintResources/StandardMacros.FlipFlop`
      (:`A`
        (set `self.RowOffset` (* (`self.Radius`) -1.0)))
      (:`B`
        (set `self.RowOffset` 0.0)))))