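; BP_Tile is a map grid tile that randomizes its own elevation as either water or land.
; Its construction script uses one random roll to pick base water height or land, with land height taken from a second, clamped roll.
; That height, scaled by Strength plus Offset, shifts the Tile component vertically and feeds the materials' Elevation parameter.
; The event graph holds only disabled placeholder events.
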(fn `UserConstructionScript`
  (bind _returnvalue (`KismetMathLibrary.RandomFloatInRange` -1.0 1.0))
  (bind _tile (`self.Tile`))
  ;[1 1 1] Calculate Height
  (if (<= _returnvalue 0.0)
    (set `self.Height` (`self.Base Water Height`))
    (else
      (set `self.Height` (`KismetMathLibrary.FClamp` _returnvalue 0.1))))
  (`SceneComponent.K2_SetWorldLocation` _tile (+ (`SceneComponent.K2_GetComponentLocation` _tile) (`KismetMathLibrary.MakeVector` 0.0 0.0 (+ (* (`self.Strength`) (`self.Height`)) (`self.Offset`)))) false false)
  (`MeshComponent.SetScalarParameterValueOnMaterials` (`self.Tile`) "Elevation" (`self.Height`)))