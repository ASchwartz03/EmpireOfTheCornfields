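; BP_troopMover issues context-sensitive orders to a group of troops based on what the camera looks at.
; giveCommand traces forward from the camera and branches on the hit actor: the hex grid moves troops, an attack target sets attack, and a resource harvester sends builders to gather.
; Vehicle and selectable building branches loop over troops without issuing orders.
; A separate pass-through event relays a resource node to a unit's SetIsWorkingMessage.
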(event `ResourcePassThroughSetIsWorking`
  (params (Unit :type "Actor Object Reference") (`Resource Node` :type "Actor Object Reference"))
  (message `/Game/Building/Interfaces/ResourceInterface/BPI_ResourceInterface.SetIsWorking` Unit `Resource Node`))

(event `giveCommand`
  (params (troops :type "Array of Actor Object Reference") (camera :type "/Game/Camera3/BP_CameraPawn3 Object Reference"))
  (bind _camera (`/Game/Camera3/BP_CameraPawn3.Camera` camera))
  (bind _returnvalue (`SceneComponent.K2_GetComponentLocation` _camera))
  (set `self.Troops` troops)
  (bind _outhit (`KismetSystemLibrary.LineTraceSingleForObjects` _returnvalue (+ _returnvalue (* (`SceneComponent.GetForwardVector` _camera) 2500.0)) (`|MakeArray` "ObjectTypeQuery2" :!type "EObjectTypeQuery Enum")))
  (bind (_bblockinghit _binitialoverlap _time _distance _location _impactpoint _normal _impactnormal _physmat _hitactor) (`GameplayStatics.BreakHitResult` _outhit))
  (cast `/Game/Map_Grid/BP_HexGrid` _hitactor
    (:`then`
      (for _array_element (`self.Troops`)
        (bind _astroop_1 (cast `/Game/Interface/Troops/Troop1` _array_element))
        (`/Game/Interface/Troops/Troop1.setStateMoveToLocation` _astroop_1 _impactpoint)))
    (:`CastFailed`
      (bind _asbp_attack_this (cast `/Game/TemporaryStandinClasses/BP_attackThis` _hitactor)
        (:`then`
          (for _array_element_2 (`self.Troops`)
            (bind _astroop_1_2 (cast `/Game/Interface/Troops/Troop1` _array_element_2))
            (`/Game/Interface/Troops/Troop1.setStateAttack` _astroop_1_2 _asbp_attack_this)))
        (:`CastFailed`
          (cast `/Game/TroopMover/BP_vehicle` _hitactor
            (:`then`
              (for _array_element_3 (`self.Troops`)
                (cast `/Game/Interface/Troops/Troop1` _array_element_3)))
            (:`CastFailed`
              (bind _asbp_resources_harvester (cast `/Game/Building/Resources/BP_ResourcesHarvester` _hitactor)
                (:`then`
                  (for _array_element_4 (`self.Troops`)
                    (bind _asbp_builder (cast `/Game/Interface/Troops/BP_Builder` _array_element_4))
                    (`/Game/Interface/Troops/BP_Builder.setStateGather` _asbp_builder _asbp_resources_harvester)))
                (:`CastFailed`
                  (cast `/Game/Building/Buildings/BP_BuildingSelectable` _hitactor)
                  (for _ (`self.Troops`)
                    _))))))))))

(fn `UserConstructionScript`)