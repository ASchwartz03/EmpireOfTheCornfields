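; BP_tank is the tank troop, a child Blueprint of a parent troop class that shows its current state with Paper2D flipbooks.
; Its construction script sets the tank TroopType after calling the parent.
; The idle, in-vehicle, attack and move-to-location state overrides call the parent, then swap the flipbook, with in-vehicle reusing the idle animation.
; The event graph holds only disabled default events.
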(fn `setStateAttack`
  (params (enemy :type "/Game/TemporaryStandinClasses/BP_attackThis Object Reference"))
  (`parent.setStateAttack` enemy)
  (`PaperFlipbookComponent.SetFlipbook` (`self.PaperFlipbook`) "/Game/ArtAssets/flipbooks/tank/attack/Tank_Attack_FB.Tank_Attack_FB"))

(fn `setStateIdle`
  (`parent.setStateIdle`)
  (`PaperFlipbookComponent.SetFlipbook` (`self.PaperFlipbook`) "/Game/ArtAssets/flipbooks/tank/idle/Tank_Idle_FB.Tank_Idle_FB"))

(fn `setStateInVehicle`
  (params (vehicle :type "/Game/TroopMover/BP_vehicle Object Reference"))
  (`parent.setStateInVehicle` vehicle)
  (`PaperFlipbookComponent.SetFlipbook` (`self.PaperFlipbook`) "/Game/ArtAssets/flipbooks/tank/idle/Tank_Idle_FB.Tank_Idle_FB"))

(fn `setStateMoveToLocation`
  (params (location :type "Vector Structure"))
  (`parent.setStateMoveToLocation` location)
  (`PaperFlipbookComponent.SetFlipbook` (`self.PaperFlipbook`) "/Game/ArtAssets/flipbooks/tank/walk/Tank_Walk_FB.Tank_Walk_FB"))

(fn `UserConstructionScript`
  (`parent.UserConstructionScript`)
  (set `self.troopType` "NewEnumerator3"))