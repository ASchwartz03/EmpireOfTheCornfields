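; BP_Builder is a worker troop that gathers beer, cash and dip and can fight enemies.
; Tick switches on State to idle, move, gather or attack with cooldown-timed damage, using AIMoveTo with slight random offsets.
; A separate DropOff event walks it to BP_Trailer, banks its load in the GMB_Camera3 game mode, then resumes gathering.
; BeginPlay snaps movement to a plane below the hex grid's origin.
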(event `self.ReceiveBeginPlay`
  (bind _floatingpawnmovement (`self.FloatingPawnMovement`))
  ;[1 1 1] Event Begin Play
  (`parent.ReceiveBeginPlay`)
  (bind _returnvalue (`GameplayStatics.GetActorOfClass` "/Game/Map_Grid/BP_HexGrid.BP_HexGrid_C"))
  (`MovementComponent.SetPlaneConstraintOrigin` _floatingpawnmovement (+ (`self.K2_GetActorLocation` _returnvalue) (0.0 0.0 -220.0)))
  (`MovementComponent.SnapUpdatedComponentToPlane` _floatingpawnmovement))

(event `self.ReceiveActorBeginOverlap`
  (params (OtherActor :type "Actor Object Reference"))
  ;[1 1 1] Overlap
  (`parent.ReceiveActorBeginOverlap` OtherActor))

(event `self.ReceiveTick`
  (params (DeltaSeconds :type "Float (single-precision)"))
  ;[1 1 1] Overlap
  (`parent.ReceiveTick` DeltaSeconds)
  (switch `/Game/Interface/ENUM_Troop1State` (`self.state`)
    (:`NewEnumerator0`
      ;;[1 1 1] Troop Movement Functions
      (`self.idleTick`))
    (:`NewEnumerator1`
      (`self.AttackTick_B`))
    (:`NewEnumerator2`
      (`self.Move to Location`))
    (:`NewEnumerator3`
      (`self.Gather2`))))

(event `Move to Location`
  ;[1 1 1] Move to Location
  (set `self.ResourceHarvester` null)
  (if (> (`KismetMathLibrary.Vector_Distance` (`self.K2_GetActorLocation`) (`self.Location`)) 120.0)
    (`|AIMoveTo` self (+ (`self.Location`) (* (`KismetMathLibrary.RandomUnitVector`) 10.0)) null 100.0)))

(event `AttackTick_B`
  ;[1 1 1] Attack Tick
  (`/Engine/EditorBlueprintResources/StandardMacros.IsValid` (`self.enemy`)
    (:`Is Valid`
      (set `self.ResourceHarvester` null)
      (if (> (`KismetMathLibrary.Vector_Distance` (`self.K2_GetActorLocation`) (`self.K2_GetActorLocation` (`self.enemy`))) 120.0)
        (`|AIMoveTo` self (+ (`self.K2_GetActorLocation` (`self.enemy`)) (* (`KismetMathLibrary.RandomUnitVector`) 10.0)) null 100.0)
        (else
          (bind _result (`/Engine/EditorBlueprintResources/StandardMacros.DecrementInt` (`self.attackCooldown`))
            (:`  `
              (if (<= _result 0)
                (`/Game/TemporaryStandinClasses/BP_attackThis.decreaseHealth` (`self.enemy`) 5)
                (set `self.attackCooldown` (`self.maxAttackCooldown`))))))))
    (:`Is Not Valid`
      (`self.setStateIdleBuild`))))

(event `Gather2`
  ;[1 1 1] Gather
  (set `self.state` "NewEnumerator3")
  (`/Engine/EditorBlueprintResources/StandardMacros.IsValid` (`self.ResourceHarvester`)
    (:`Is Valid`
      (if (> (`KismetMathLibrary.Vector_Distance` (`self.K2_GetActorLocation`) (`self.K2_GetActorLocation` (`self.ResourceHarvester`))) 120.0)
        (set `self.HasResourceB?` true)
        (`|AIMoveTo` self (+ (`self.K2_GetActorLocation` (`self.ResourceHarvester`)) (* (`KismetMathLibrary.RandomUnitVector`) 10.0)) null 100.0)))
    (:`Is Not Valid`
      (`/Engine/EditorBlueprintResources/StandardMacros.IsValid` (`self.enemy`)
        (:`Is Valid`
          (`self.AttackTick_B`))
        (:`Is Not Valid`
          (`self.setStateIdleBuild`))))))

(event `Drop Off`
  ;[1 1 1] Drop Off
  (`/Engine/EditorBlueprintResources/StandardMacros.IsValid` (`self.ResourceHarvester`)
    (:`Is Valid`
      (`self.setStateDrop`)
      (bind _returnvalue (`GameplayStatics.GetActorOfClass` "/Game/Building/Buildings/Trailer/BP_Trailer.BP_Trailer_C"))
      (`/Engine/EditorBlueprintResources/StandardMacros.IsValid` _returnvalue
        (:`Is Valid`
          (`|AIMoveTo` self (0.0 0.0 0.0) _returnvalue 5.0 true
            (:`OnSuccess`
              (`self.Beer Drop Off`)
              (`self.Cash Drop Off`)
              (`self.Dip Drop Off`)
              (set `self.HasResourceB?` false)
              (`/Engine/EditorBlueprintResources/StandardMacros.IsValid` (`self.ResourceHarvester`)
                (:`Is Valid`
                  (`self.Gather2`))
                (:`Is Not Valid`
                  (`/Engine/EditorBlueprintResources/StandardMacros.IsValid` (`self.enemy`)
                    (:`Is Valid`
                      (`self.AttackTick_B`))
                    (:`Is Not Valid`
                      (`self.setStateIdleBuild`))))))))))))

(fn `Beer Drop Off`
  (bind _asgmb_camera_3 (cast `/Game/Camera3/GMB_Camera3` (`GameplayStatics.GetGameMode`)))
  (set `/Game/Camera3/GMB_Camera3.BeerInventory` (+ (`/Game/Camera3/GMB_Camera3.BeerInventory` _asgmb_camera_3) (`self.Beer`)) _asgmb_camera_3)
  (set `self.Beer` 0))

(fn `Cash Drop Off`
  (bind _asgmb_camera_3 (cast `/Game/Camera3/GMB_Camera3` (`GameplayStatics.GetGameMode`)))
  (set `/Game/Camera3/GMB_Camera3.CashInventory` (+ (`/Game/Camera3/GMB_Camera3.CashInventory` _asgmb_camera_3) (`self.Cash`)) _asgmb_camera_3)
  (set `self.Cash` 0))

(fn `decreasehealth_Build`
  (params (health :type Integer))
  (bind _output_get (set `self.health` (- (`self.health`) health)))
  (if (<= _output_get 0)
    (`self.K2_DestroyActor`)))

(fn `Dip Drop Off`
  (bind _asgmb_camera_3 (cast `/Game/Camera3/GMB_Camera3` (`GameplayStatics.GetGameMode`)))
  (set `/Game/Camera3/GMB_Camera3.DipInventory` (+ (`/Game/Camera3/GMB_Camera3.DipInventory` _asgmb_camera_3) (`self.Dip`)) _asgmb_camera_3)
  (set `self.Dip` 0))

(fn `idleTick`)

(fn `setStateAttack`
  (params (enemy :type "/Game/TemporaryStandinClasses/BP_attackThis Object Reference"))
  (set `self.enemy` enemy)
  (set `self.state` "NewEnumerator1"))

(fn `setStateDrop`
  (set `self.state` "NewEnumerator4"))

(fn `setStateGather`
  (params (ResourceHarvester :type "/Game/Building/Resources/BP_ResourcesHarvester Object Reference"))
  (set `self.ResourceHarvester` ResourceHarvester)
  (set `self.state` "NewEnumerator3"))

(fn `setStateIdleBuild`
  (set `self.state` "NewEnumerator0"))

(fn `setStateMoveToLocationBuild`
  (params (location :type "Vector Structure"))
  (set `self.Location` location)
  (set `self.state` "NewEnumerator2"))

(fn `UserConstructionScript`
  (`parent.UserConstructionScript`))