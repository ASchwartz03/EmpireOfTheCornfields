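; Gunner troop Blueprint, a 2D flipbook child of a parent troop class that supplies the gunner's animations and attack sound.
; The construction script sets its troop type.
; Overrides of the attack, idle, in-vehicle and move-to-location state setters call the parent, then swap the Paper2D flipbook, with the vehicle state reusing idle.
; Attack also plays a non-spatial shotgun cue, and the event graph holds no active logic.
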(fn `setStateAttack`
  (params (enemy :type "/Game/TemporaryStandinClasses/BP_attackThis Object Reference"))
  (`parent.setStateAttack` enemy)
  (`PaperFlipbookComponent.SetFlipbook` (`self.PaperFlipbook`) "/Game/ArtAssets/flipbooks/gunner/attack/gunner_Attack_FB.gunner_Attack_FB")
  (`GameplayStatics.PlaySound2D` "/Game/Audio/Combat___Weapon/Shotgun_Cue.Shotgun_Cue" 1.0 1.0 0.0 null null))

(fn `setStateIdle`
  (`parent.setStateIdle`)
  (`PaperFlipbookComponent.SetFlipbook` (`self.PaperFlipbook`) "/Game/ArtAssets/flipbooks/gunner/idle/gunner_Idle_FB.gunner_Idle_FB"))

(fn `setStateInVehicle`
  (params (vehicle :type "/Game/TroopMover/BP_vehicle Object Reference"))
  (`parent.setStateInVehicle` vehicle)
  (`PaperFlipbookComponent.SetFlipbook` (`self.PaperFlipbook`) "/Game/ArtAssets/flipbooks/gunner/idle/gunner_Idle_FB.gunner_Idle_FB"))

(fn `setStateMoveToLocation`
  (params (location :type "Vector Structure"))
  (`parent.setStateMoveToLocation` location)
  (`PaperFlipbookComponent.SetFlipbook` (`self.PaperFlipbook`) "/Game/ArtAssets/flipbooks/gunner/walk/gunner_Walk_FB.gunner_Walk_FB"))

(fn `UserConstructionScript`
  (`parent.UserConstructionScript`)
  (set `self.troopType` "NewEnumerator1"))