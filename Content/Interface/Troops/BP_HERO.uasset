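; BP_HERO is the hero troop pawn, which moves on a plane offset below the BP_HexGrid and fights a target enemy.
; Setter functions switch a Tick-driven state machine between an empty Idle, Move to Location and Attack.
; Attack chases via AI MoveTo with slight random offset, then deals damage on a tick-counted cooldown, idling once the enemy is invalid.
; A super event deals heavier damage, and depleted health destroys the hero.
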(event `self.ReceiveBeginPlay`
  (bind _floatingpawnmovement (`self.FloatingPawnMovement`))
  (`parent.ReceiveBeginPlay`)
  (bind _returnvalue (`GameplayStatics.GetActorOfClass` "/Game/Map_Grid/BP_HexGrid.BP_HexGrid_C"))
  (`MovementComponent.SetPlaneConstraintOrigin` _floatingpawnmovement (+ (`self.K2_GetActorLocation` _returnvalue) (0.0 0.0 -220.0)))
  (`MovementComponent.SnapUpdatedComponentToPlane` _floatingpawnmovement))

(event `self.ReceiveActorBeginOverlap`
  (params (OtherActor :type "Actor Object Reference"))
  (`parent.ReceiveActorBeginOverlap` OtherActor))

(event `self.ReceiveTick`
  (params (DeltaSeconds :type "Float (single-precision)"))
  (`parent.ReceiveTick` DeltaSeconds)
  (switch `/Game/Interface/ENUM_Troop1State` (`self.state`)
    (:`NewEnumerator0`
      (`self.idleTick`))
    (:`NewEnumerator1`
      (`self.AttackTick_H`))
    (:`NewEnumerator2`
      (`self.Move to Location`))))

(event `self.attackTick`)

(event `Move to Location`
  (if (> (`KismetMathLibrary.Vector_Distance` (`self.K2_GetActorLocation`) (`self.Location`)) 120.0)
    (`|AIMoveTo` self (+ (`self.Location`) (* (`KismetMathLibrary.RandomUnitVector`) 10.0)) null 100.0)))

(event `AttackTick_H`
  (`/Engine/EditorBlueprintResources/StandardMacros.IsValid` (`self.enemy`)
    (:`Is Valid`
      (if (> (`KismetMathLibrary.Vector_Distance` (`self.K2_GetActorLocation`) (`self.K2_GetActorLocation` (`self.enemy`))) 120.0)
        (`|AIMoveTo` self (+ (`self.K2_GetActorLocation` (`self.enemy`)) (* (`KismetMathLibrary.RandomUnitVector`) 10.0)) null 100.0)
        (else
          (bind _result (`/Engine/EditorBlueprintResources/StandardMacros.DecrementInt` (`self.attackCooldown`))
            (:`  `
              (if (<= _result 0)
                (`/Game/TemporaryStandinClasses/BP_attackThis.decreaseHealth` (`self.enemy`) 5)
                (set `self.attackCooldown` (`self.maxAttackCooldown`))))))))
    (:`Is Not Valid`
      (`self.setStateIdleHero`))))

(event `Hero Supder`
  (params (HeroSuperCalled :type Boolean))
  (`/Game/TemporaryStandinClasses/BP_attackThis.decreaseHealth` (`self.enemy`) 20))

(fn `decreasehealth_Hero`
  (params (health :type Integer))
  (bind _output_get (set `self.health` (- (`self.health`) health)))
  (if (<= _output_get 0)
    (`self.K2_DestroyActor`)))

(fn `idleTick`)

(fn `setStateAttack`
  (params (enemy :type "/Game/TemporaryStandinClasses/BP_attackThis Object Reference"))
  (set `self.enemy` enemy)
  (set `self.state` "NewEnumerator1"))

(fn `setStateIdleHero`
  (set `self.state` "NewEnumerator0"))

(fn `setStateMoveToLocationHero`
  (params (location :type "Vector Structure"))
  (set `self.Location` location)
  (set `self.state` "NewEnumerator2"))

(fn `UserConstructionScript`
  (`parent.UserConstructionScript`))