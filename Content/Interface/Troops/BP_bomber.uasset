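; Bomber troop Blueprint, a child of a troop base with a Paper2D flipbook, that demolishes buildings.
; The destroyBuilding event walks it to the target, plays the attack flipbook, then after a fixed delay destroys the building and returns to idle.
; Overrides of the parent's attack, idle, vehicle and move state setters raise an Interrupted flag, which cancels demolition if set during that delay.
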(event `destroyBuilding`
  (params (building :type "/Game/Building/Buildings/BP_BuildingSelectable Object Reference"))
  (bind _building (`self.Building`))
  (set `self.Building` building)
  (`|AIMoveTo` self (0.0 0.0 0.0) (`self.Building`) 100.0
    (:`OnSuccess`
      (`PaperFlipbookComponent.SetFlipbook` (`self.PaperFlipbook`) "/Game/ArtAssets/flipbooks/bomber/attack/Bomber_Attack_FB.Bomber_Attack_FB")
      (set `self.interrupted` false)
      (`KismetSystemLibrary.Delay` 5.0)
      (if (not (`self.interrupted`))
        (`/Engine/EditorBlueprintResources/StandardMacros.IsValid` _building
          (:`Is Valid`
            (`self.K2_DestroyActor` _building))
          (:`Is Not Valid`
            _))
        (set `self.Building` null)
        (`self.setStateIdle`)))))

(fn `setStateAttack`
  (params (enemy :type "/Game/TemporaryStandinClasses/BP_attackThis Object Reference"))
  (`parent.setStateAttack` enemy)
  (set `self.interrupted` true))

(fn `setStateIdle`
  (`parent.setStateIdle`)
  (set `self.interrupted` true))

(fn `setStateInVehicle`
  (params (vehicle :type "/Game/TroopMover/BP_vehicle Object Reference"))
  (`parent.setStateInVehicle` vehicle)
  (set `self.interrupted` true))

(fn `setStateMoveToLocation`
  (params (location :type "Vector Structure"))
  (`parent.setStateMoveToLocation` location)
  (set `self.interrupted` true))

(fn `UserConstructionScript`
  (`parent.UserConstructionScript`)
  (set `self.troopType` "NewEnumerator0"))